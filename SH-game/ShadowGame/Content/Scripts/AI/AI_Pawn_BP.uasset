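; Enemy AI pawn that spots the player, follows, fights, takes hits and dies with slow motion.
; Sight and Tick distance checks against a randomized range switch Follow and Combat states, mirrored with other values to the AI controller's Blackboard.
; A randomly timed CombatLoop picks weighted combat sub-states, while hits interrupt it and apply damage.
; Tick also checks health and ground; helpers toggle an attack indicator and outline, and a timer plays grunts.
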(event `self.ReceiveBeginPlay`
  (`self.SpawnDefaultController`)
  (set `self.StartLocation` (`self.K2_GetActorLocation`))
  (`self.SetFloatBlackBoard` "MaxWanderDistance" (`self.MaxWanderDistance`))
  (`BlackboardComponent.SetValueAsVector` (`AIBlueprintHelperLibrary.GetBlackboard` (`AIBlueprintHelperLibrary.GetAIController` self)) "StartLocation" (`self.StartLocation`))
  (`self.SetEnumStateBlackBoard` (`self.CurrentState`))
  (`self.SetEnumCombatStateBlackBoard` (`self.CurrentCombatState`))
  (bind _output_get (set `self.DistanceToPlayer` (+ (* (`KismetMathLibrary.RandomFloat`) 100.0) 350.0)))
  (`self.SetFloatBlackBoard` "DistanceToPlayer" _output_get)
  (`KismetSystemLibrary.K2_SetTimer` null "Sound" (`KismetMathLibrary.RandomFloatInRange` 5.0 10.0)))

(event `self.PawnSensing.OnSeePawn`
  (params (Pawn :type "Pawn Object Reference"))
  (if (== Pawn (`GameplayStatics.GetPlayerPawn` 0))
    (`/Engine/EditorBlueprintResources/StandardMacros.IsValid` (`self.EnemyPawn`)
      (:`Is Not Valid`
        (bind _output_get (set `self.EnemyPawn` Pawn))
        (`BlackboardComponent.SetValueAsObject` (`AIBlueprintHelperLibrary.GetBlackboard` (`AIBlueprintHelperLibrary.GetAIController` self)) "EnemyPawn" _output_get)
        (bind _output_get_2 (set `self.CurrentState` "NewEnumerator1"))
        (`self.SetEnumStateBlackBoard` _output_get_2)))))

(event `self.ReceiveTick`
  (params (DeltaSeconds :type "Float (single-precision)"))
  (bind _enemypawn (`self.EnemyPawn`))
  (bind _enemypawn_2 (`self.EnemyPawn`))
  (bind (_returnvalue_roll _returnvalue_pitch _returnvalue_yaw) (`KismetMathLibrary.BreakRotator` (`KismetMathLibrary.FindLookAtRotation` (`self.K2_GetActorLocation`) (`self.K2_GetActorLocation` (`self.EnemyPawn`)))))
  (bind (_returnvalue_roll_2 _returnvalue_pitch_2 _returnvalue_yaw_2) (`KismetMathLibrary.BreakRotator` (`KismetMathLibrary.FindLookAtRotation` (`self.K2_GetActorLocation`) (`self.K2_GetActorLocation` (`self.EnemyPawn`)))))
  (`self.CheckHealth`)
  (`self.CheckGround`)
  (switch `/Game/Scripts/AI/EnemyStates` (`self.CurrentState`)
    (:`NewEnumerator1`
      (`/Engine/EditorBlueprintResources/StandardMacros.IsValid` _enemypawn
        (:`Is Valid`
          (`self.K2_SetActorRotation` (`KismetMathLibrary.RInterpTo` (`self.K2_GetActorRotation`) (`KismetMathLibrary.MakeRotator` 0.0 0.0 _returnvalue_yaw_2) (`GameplayStatics.GetWorldDeltaSeconds`) 15.0))
          (if (<= (`KismetMathLibrary.Vector_Distance` (`self.K2_GetActorLocation` _enemypawn) (`self.K2_GetActorLocation`)) (+ (`self.DistanceToPlayer`) 50.0))
            (bind _output_get (set `self.CurrentState` "NewEnumerator2"))
            (`self.SetEnumStateBlackBoard` _output_get)))))
    (:`NewEnumerator2`
      (`/Engine/EditorBlueprintResources/StandardMacros.IsValid` _enemypawn_2
        (:`Is Valid`
          (if (> (`KismetMathLibrary.Vector_Distance` (`self.K2_GetActorLocation` _enemypawn_2) (`self.K2_GetActorLocation`)) (+ (`self.DistanceToPlayer`) 50.0))
            (if (!= (`self.CurrentCombatState`) 2)
              (bind _output_get_2 (set `self.CurrentState` "NewEnumerator1"))
              (`self.SetEnumStateBlackBoard` _output_get_2))
            (elif (`KismetSystemLibrary.K2_IsTimerActive` null "CombatLoop")
              (if (!= (`self.CurrentCombatState`) 2)
                (`self.K2_SetActorRotation` (`KismetMathLibrary.RInterpTo` (`self.K2_GetActorRotation`) (`KismetMathLibrary.MakeRotator` 0.0 0.0 _returnvalue_yaw) (`GameplayStatics.GetWorldDeltaSeconds`) 15.0)))
              (elif (!= (`self.CurrentCombatState`) 2)
                (`KismetSystemLibrary.K2_SetTimer` null "CombatLoop" (`self.Random float` 0.5 2.0) false true)))))))))

(event `/Game/Scripts/AI/EnemyInterface.Hit`
  (bind _returnvalue (`KismetMathLibrary.MakeRotator` (* (- (`KismetMathLibrary.RandomFloat`) 0.5) 360.0) (* (- (`KismetMathLibrary.RandomFloat`) 0.5) 360.0) (* (- (`KismetMathLibrary.RandomFloat`) 0.5) 360.0)))
  (bind _returnvalue_2 (+ (`self.K2_GetActorLocation`) (* (* (`KismetMathLibrary.MakeVector` (- (`KismetMathLibrary.RandomFloat`) 0.5) (- (`KismetMathLibrary.RandomFloat`) 0.5) (- (`KismetMathLibrary.RandomFloat`) 0.5)) 2.0) (30.0 30.0 30.0))))
  (if (!= (`self.CurrentState`) 3)
    (`/Engine/EditorBlueprintResources/StandardMacros.IsValid` (`self.EnemyPawn`)
      (:`Is Valid`
        (`KismetSystemLibrary.K2_ClearTimer` null "CombatLoop")
        (`KismetSystemLibrary.K2_PauseTimer` null "CombatLoop")
        (`self.TakeDamage` 30.0)
        (set `self.CurrentState` "NewEnumerator3")
        (`self.SetEnumStateBlackBoard` "NewEnumerator3")
        (`GameplayStatics.SpawnEmitterAtLocation` "/Game/Scripts/NiagaraTest/EnemyHit.EnemyHit" _returnvalue_2 _returnvalue (7.0 7.0 7.0))
        (`GameplayStatics.SpawnEmitterAtLocation` "/Game/Scripts/NiagaraTest/Shockwave.Shockwave" _returnvalue_2 _returnvalue (`KismetMathLibrary.MakeVector` 3.0 3.0 3.0))
        (`KismetSystemLibrary.PrintString` "Enemy Got Hit")))))

(fn `ActivateHiglight`
  (`MeshComponent.SetOverlayMaterial` (`self.SkeletalMesh`) "/Game/Scripts/Outlines/EnemyOutline.EnemyOutline"))

(fn `CheckGround`
  (bind _returnvalue (`self.K2_GetActorLocation`))
  (bind (_outhits _returnvalue_2) (`KismetSystemLibrary.LineTraceMulti` _returnvalue (+ _returnvalue (0.0 0.0 -400.0)) "TraceTypeQuery2"))
  (if (not _returnvalue_2)
    (`self.Die`)))

(fn `CheckHealth`
  (if (<= (`self.CurrentHealth`) 0.0)
    (`self.Destroy`)))

(fn `CombatLoop`
  (locals (NextState :type "Float (double-precision)"))
  (bind _output_get (set `local.NextState` (`self.Random float` 0.0 100.0)))
  (if (< _output_get 50.0)
    (set `self.CurrentCombatState` "NewEnumerator1")
    (elif (< _output_get 60.0)
      (set `self.CurrentCombatState` "NewEnumerator0")
      (else
        (set `self.CurrentCombatState` "NewEnumerator2"))))
  (`self.SetEnumCombatStateBlackBoard` (`self.CurrentCombatState`)))

(fn `DeactivateHighlight`
  (`MeshComponent.SetOverlayMaterial` (`self.SkeletalMesh`) "/Game/Scripts/Outlines/Nothing.Nothing"))

(fn `Destroy`
  (`GameplayStatics.SpawnEmitterAtLocation` "/Game/Scripts/NiagaraTest/EnemyDie.EnemyDie" (`self.K2_GetActorLocation`) (struct) (2.0 2.0 2.0))
  (`GameplayStatics.SetGlobalTimeDilation` 0.2)
  (bind _asplayer_pawn (cast `/Game/Scripts/Player/PlayerPawn` (`self.EnemyPawn`)))
  (`/Game/Scripts/Player/PlayerPawn.ResetTime` _asplayer_pawn 0.035)
  (`self.K2_DestroyActor`)
  (`KismetSystemLibrary.PrintString` "DestroySelf"))

(fn `Die`
  (if (`KismetSystemLibrary.K2_IsTimerActive` null "Destroy")
    (`self.Destroy`)))

(fn `HideAttackIndicator`
  (`SceneComponent.SetVisibility` (`self.MaterialBillboard`) false false))

(fn `SetEnumCombatStateBlackBoard`
  (params (Value :type "/Game/Scripts/AI/EnemyCombatStates Enum" :default "NewEnumerator0"))
  (`BlackboardComponent.SetValueAsEnum` (`AIBlueprintHelperLibrary.GetBlackboard` (`AIBlueprintHelperLibrary.GetAIController` self)) "CurrentCombatState" Value))

(fn `SetEnumStateBlackBoard`
  (params (Value :type "/Game/Scripts/AI/EnemyStates Enum" :default "NewEnumerator0"))
  (`BlackboardComponent.SetValueAsEnum` (`AIBlueprintHelperLibrary.GetBlackboard` (`AIBlueprintHelperLibrary.GetAIController` self)) "CurrentState" Value))

(fn `SetFloatBlackBoard`
  (params (Name :type Name) (Value :type "Float (double-precision)"))
  (`BlackboardComponent.SetValueAsFloat` (`AIBlueprintHelperLibrary.GetBlackboard` (`AIBlueprintHelperLibrary.GetAIController` self)) (`KismetSystemLibrary.MakeLiteralName` Name) Value))

(fn `ShowAttackIndicator`
  (`SceneComponent.SetVisibility` (`self.MaterialBillboard`) true false))

(fn `Sound`
  (`KismetSystemLibrary.K2_SetTimer` null "Sound" (`KismetMathLibrary.RandomFloatInRange` 5.0 15.0))
  (`GameplayStatics.PlaySoundAtLocation` "/Game/Scripts/Sounds/GruntCue.GruntCue" (`self.K2_GetActorLocation`) (struct) 1.0 1.0 0.0 null null null null))

(fn `TakeDamage`
  (params (damage :type "Float (double-precision)"))
  (set `self.CurrentHealth` (- (`self.CurrentHealth`) damage)))

(fn `UserConstructionScript`)