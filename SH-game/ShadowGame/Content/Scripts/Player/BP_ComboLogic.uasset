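; BP_ComboLogic tracks the player's combo count and reports it to the UI overlay on the player pawn.
; IncreaseCombo bumps the count, restarts a 1.5-second ResetCombo timer, updates the UI and sets CurrentOpacity to full.
; When the timer expires, ResetCombo zeroes the count and updates the UI.
; Tick fades CurrentOpacity from the timer's remaining time, or holds it at half when no timer is active.
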(event `self.ReceiveTick`
  (params (DeltaSeconds :type "Float (single-precision)"))
  (if (`KismetSystemLibrary.K2_IsTimerActive` null "ResetCombo")
    (set `self.CurrentOpacity` (- 1.0 (/ (/ (- 1.5 (`KismetSystemLibrary.K2_GetTimerRemainingTime` null "ResetCombo")) 1.5) 1.5)))
    (else
      (set `self.CurrentOpacity` 0.5))))

(fn `IncreaseCombo`
  (`KismetSystemLibrary.K2_PauseTimer` null "ResetCombo")
  (set `self.CurrentCombo` (+ (`self.CurrentCombo`) 1))
  (`KismetSystemLibrary.K2_SetTimer` null "ResetCombo" 1.5)
  (bind _asplayer_pawn (cast `/Game/Scripts/Player/PlayerPawn` (`GameplayStatics.GetPlayerPawn` 0)))
  (bind _asui (cast `/Game/Scripts/UI/UI` (`/Game/Scripts/Player/PlayerPawn.UI_Overlay` _asplayer_pawn)))
  (`/Game/Scripts/UI/UI.IncreaseCombo` _asui)
  (`/Game/Scripts/UI/UI.SetCombo` _asui (`self.CurrentCombo`))
  (set `self.CurrentOpacity` 1.0))

(fn `ResetCombo`
  (set `self.CurrentCombo` 0)
  (bind _asplayer_pawn (cast `/Game/Scripts/Player/PlayerPawn` (`GameplayStatics.GetPlayerPawn` 0)))
  (bind _asui (cast `/Game/Scripts/UI/UI` (`/Game/Scripts/Player/PlayerPawn.UI_Overlay` _asplayer_pawn)))
  (`/Game/Scripts/UI/UI.SetCombo` _asui (`self.CurrentCombo`)))

(fn `UserConstructionScript`)